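; Health Blueprint for characters that tracks current health and death state.
; BeginPlay sets current health from the starting value, and a Damage event subtracts from it until death, ignoring further hits afterward.
; Reaching zero clamps health, sets the death flag and calls Death; non-lethal hits call Damage, with both outcomes printed to screen for debugging.
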(event `self.ReceiveBeginPlay`
  (set `self.CurrentHealth` (`self.StartHealth`)))

(event `Event Damage`
  (params (Damage :type "Float (double-precision)"))
  (if (not (`self.IsDeath`))
    (set `self.CurrentHealth` (- (`self.CurrentHealth`) Damage))
    (if (<= (`self.CurrentHealth`) 0.0)
      (set `self.IsDeath` true)
      (set `self.CurrentHealth` 0.0)
      (`self.Death`)
      (`KismetSystemLibrary.PrintString` "Death")
      (else
        (`self.Damage`)
        (`KismetSystemLibrary.PrintString` (`KismetStringLibrary.Conv_DoubleToString` (`self.CurrentHealth`)))))))