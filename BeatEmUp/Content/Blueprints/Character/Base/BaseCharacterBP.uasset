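; Base character Blueprint for a beat 'em up, handling facing, melee attacks, hit boxes and Enhanced Input mapping contexts.
; Attack locks movement and further attacks, flags the animation Blueprint and buffers the hand used.
; ActiveHitBoxAnimation toggles that hand's collision box and its visibility, while ResetAttack restores control and disables all boxes.
; Facing flips by rotating the mesh according to the direction's sign.
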(event `self.ReceiveBeginPlay`
  (`self.GetAnimation`)
  (`self.DeactiveHitBoxes`))

(event `ResetAttack`
  (`self.ResetCombo`))

(event `ActiveHitBoxAnimation`
  (params (IsActive :type Boolean))
  (`self.ActiveHitBox` (`self.AttackHitBoxBuffer`) IsActive))

(fn `ActiveHitBox`
  (params (AttackType :type "/Game/Blueprints/Enums/AttackType Enum" :default "NewEnumerator3") (IsActive :type Boolean))
  (locals (BoxCollision :type "BoxComponent Object Reference"))
  (`|ExecutionSequence`
    (:`then_0`
      (switch `/Game/Blueprints/Enums/AttackType` AttackType
        (:`NewEnumerator0`
          (set `local.BoxCollision` (`self.HitBoxLeftHand`)))
        (:`NewEnumerator1`
          (set `local.BoxCollision` (`self.HitBoxRightHand`)))
        (:`NewEnumerator2`
          (set `local.BoxCollision` (`self.HitBoxElbow`)))))
    (:`then_1`
      (if IsActive
        (`PrimitiveComponent.SetCollisionEnabled` (`local.BoxCollision`) "QueryOnly")
        (`SceneComponent.SetVisibility` (`local.BoxCollision`) true false)
        (else
          (`PrimitiveComponent.SetCollisionEnabled` (`local.BoxCollision`) "NoCollision")
          (`SceneComponent.SetVisibility` (`local.BoxCollision`) false false))))))

(fn `Attack`
  (params (NewParam :type "/Game/Blueprints/Enums/InputType Enum" :default "NewEnumerator2"))
  (if (`self.IsMaybeAttack`)
    (set `self.IsMaybeAttack` false)
    (set `self.IsMaybeMoving` false)
    (set `/Game/Blueprints/Character/BeatEmUpCharacterAnimationBP.IsAttack` true (`self.Animation`))
    (switch `/Game/Blueprints/Enums/InputType` NewParam
      (:`NewEnumerator0`
        (set `/Game/Blueprints/Character/BeatEmUpCharacterAnimationBP.IsAttackLeftHand` true (`self.Animation`))
        (set `self.AttackHitBoxBuffer` "NewEnumerator0"))
      (:`NewEnumerator1`
        (set `/Game/Blueprints/Character/BeatEmUpCharacterAnimationBP.IsAttackRightHand` true (`self.Animation`))
        (set `self.AttackHitBoxBuffer` "NewEnumerator1")))))

(fn `ChangeMappingInput`
  (params (Mapping :type "InputMappingContext Object Reference"))
  (bind _asplayer_controller (cast `PlayerController` (`self.GetController`)))
  (message `EnhancedInputSubsystemInterface.AddMappingContext` (pcsubsystem `EnhancedInputLocalPlayerSubsystem` _asplayer_controller) Mapping 0 (struct)))

(fn `CheackFlip`
  (params (Direction :type "Float (double-precision)"))
  (`|ExecutionSequence`
    (:`then_0`
      (if (> Direction 0.0)
        (`self.Flip` true)))
    (:`then_1`
      (if (< Direction 0.0)
        (`self.Flip` false)))))

(fn `DeactiveHitBoxes`
  (`self.ActiveHitBox` "NewEnumerator0")
  (`self.ActiveHitBox` "NewEnumerator1")
  (`self.ActiveHitBox` "NewEnumerator2"))

(fn `Flip`
  (params (Flip :type Boolean))
  (bind _mesh (`self.Mesh`))
  (if (!= Flip (`self.IsFlip`))
    (if Flip
      (`SceneComponent.K2_SetRelativeRotation` _mesh (struct :`Yaw` -90.0) false false)
      (set `self.IsFlip` true)
      (else
        (`SceneComponent.K2_SetRelativeRotation` _mesh (struct :`Yaw` 90.0) false false)
        (set `self.IsFlip` false)))))

(fn `GetAnimation`
  (bind _asbeat_em_up_character_animation_bp (cast `/Game/Blueprints/Character/BeatEmUpCharacterAnimationBP` (`SkeletalMeshComponent.GetAnimInstance` (`self.Mesh`))))
  (set `self.Animation` _asbeat_em_up_character_animation_bp))

(fn `InitInput`
  (bind _asplayer_controller (cast `PlayerController` (`self.GetController`)))
  (message `EnhancedInputSubsystemInterface.AddMappingContext` (pcsubsystem `EnhancedInputLocalPlayerSubsystem` _asplayer_controller) "/Game/Blueprints/Input/InputMappingPlayer1BP.InputMappingPlayer1BP" 0 (struct)))

(fn `ResetCombo`
  (set `self.IsMaybeMoving` true)
  (set `self.IsMaybeAttack` true)
  (`self.DeactiveHitBoxes`))

(fn `UserConstructionScript`)