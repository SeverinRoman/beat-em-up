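; Base beat 'em up character Blueprint handling melee attacks, combos, damage, death and left/right mesh flipping.
; Attack sets animation flags and buffers inputs, which are matched against the ComboElbow sequence to chain follow-up hits while combos are allowed.
; Animation-driven events toggle hand and elbow hitboxes, whose overlaps apply damage.
; Incoming damage feeds the Health component, whose events interrupt attacks or trigger a random death animation and disable the hurtbox.
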(event `self.ReceiveBeginPlay`
  (`self.GetAnimation`)
  (`self.DeactiveHitBoxes`))

(event `ResetAttack`
  (`self.ResetCombo`))

(event `ActiveHitBoxAnimation`
  (params (IsActive :type Boolean))
  (`self.ActiveHitBox` (`self.AttackHitBoxBuffer`) IsActive))

(event `self.ReceiveAnyDamage`
  (params (Damage :type "Float (single-precision)") (DamageType :type "DamageType Object Reference") (InstigatedBy :type "Controller Object Reference") (DamageCauser :type "Actor Object Reference"))
  (if (!= DamageCauser self)
    (`/Game/Blueprints/Character/Health.Event Damage` (`self.Health`) Damage)))

(event `self.HitBoxLeftHand.OnComponentBeginOverlap`
  (params (OverlappedComponent :type "PrimitiveComponent Object Reference") (OtherActor :type "Actor Object Reference") (OtherComp :type "PrimitiveComponent Object Reference") (OtherBodyIndex :type Integer) (bFromSweep :type Boolean) (SweepResult :type "HitResult Structure (by ref)"))
  (`self.DamageOtherActor` (`self.Damage`) OtherActor))

(event `self.HitBoxRightHand.OnComponentBeginOverlap`
  (params (OverlappedComponent :type "PrimitiveComponent Object Reference") (OtherActor :type "Actor Object Reference") (OtherComp :type "PrimitiveComponent Object Reference") (OtherBodyIndex :type Integer) (bFromSweep :type Boolean) (SweepResult :type "HitResult Structure (by ref)"))
  (`self.DamageOtherActor` (`self.Damage`) OtherActor))

(event `self.HitBoxElbow.OnComponentBeginOverlap`
  (params (OverlappedComponent :type "PrimitiveComponent Object Reference") (OtherActor :type "Actor Object Reference") (OtherComp :type "PrimitiveComponent Object Reference") (OtherBodyIndex :type Integer) (bFromSweep :type Boolean) (SweepResult :type "HitResult Structure (by ref)"))
  (`self.DamageOtherActor` (`self.Damage`) OtherActor))

(event `self.Health.Damage`
  (params (CurrentHealth :type "Float (double-precision)"))
  (`self.DeactiveHitBoxes`)
  (set `/Game/Blueprints/Character/BeatEmUpCharacterAnimationBP.IsAttack` false (`self.Animation`))
  (set `/Game/Blueprints/Character/BeatEmUpCharacterAnimationBP.IsDamage` true (`self.Animation`))
  (set `self.IsMaybeMoving` false)
  (set `self.IsMaybeAttack` false))

(event `self.Health.Death`
  (`self.Death`))

(fn `ActiveHitBox`
  (params (AttackType :type "/Game/Blueprints/Enums/AttackType Enum" :default "NewEnumerator3") (IsActive :type Boolean))
  (locals (BoxCollision :type "BoxComponent Object Reference"))
  (`|ExecutionSequence`
    (:`then_0`
      (switch `/Game/Blueprints/Enums/AttackType` AttackType
        (:`NewEnumerator0`
          (set `local.BoxCollision` (`self.HitBoxLeftHand`)))
        (:`NewEnumerator1`
          (set `local.BoxCollision` (`self.HitBoxRightHand`)))
        (:`NewEnumerator2`
          (set `local.BoxCollision` (`self.HitBoxElbow`)))))
    (:`then_1`
      (if IsActive
        (`PrimitiveComponent.SetCollisionEnabled` (`local.BoxCollision`) "QueryOnly")
        (`SceneComponent.SetVisibility` (`local.BoxCollision`) true false)
        (else
          (`PrimitiveComponent.SetCollisionEnabled` (`local.BoxCollision`) "NoCollision")
          (`SceneComponent.SetVisibility` (`local.BoxCollision`) false false))))))

(fn `Attack`
  (params (InputType :type "/Game/Blueprints/Enums/InputType Enum" :default "NewEnumerator2"))
  (`self.CheackCombo` InputType)
  (if (`self.IsMaybeAttack`)
    (set `self.IsMaybeAttack` false)
    (set `self.IsMaybeMoving` false)
    (set `/Game/Blueprints/Character/BeatEmUpCharacterAnimationBP.IsAttack` true (`self.Animation`))
    (switch `/Game/Blueprints/Enums/InputType` InputType
      (:`NewEnumerator0`
        (set `/Game/Blueprints/Character/BeatEmUpCharacterAnimationBP.IsAttackLeftHand` true (`self.Animation`))
        (set `self.AttackHitBoxBuffer` "NewEnumerator0")
        (`KismetArrayLibrary.Array_Add` (`self.BufferInput`) "NewEnumerator0"))
      (:`NewEnumerator1`
        (set `/Game/Blueprints/Character/BeatEmUpCharacterAnimationBP.IsAttackRightHand` true (`self.Animation`))
        (set `self.AttackHitBoxBuffer` "NewEnumerator1")
        (`KismetArrayLibrary.Array_Add` (`self.BufferInput`) "NewEnumerator1")))))

(fn `ChangeMappingInput`
  (params (Mapping :type "InputMappingContext Object Reference"))
  (bind _asplayer_controller (cast `PlayerController` (`self.GetController`)))
  (message `EnhancedInputSubsystemInterface.AddMappingContext` (pcsubsystem `EnhancedInputLocalPlayerSubsystem` _asplayer_controller) Mapping 0 (struct)))

(fn `CheackCombo`
  (params (InputType :type "/Game/Blueprints/Enums/InputType Enum" :default "NewEnumerator2"))
  (locals (IsReplayBuffer :type Boolean :default true))
  (if (`self.IsMaybeCombo`)
    (bind _isreplay (`self.CheackInputBufferNextCombo`))
    (if _isreplay
      (bind _output_get (set `self.CounterCombo` (+ (`self.CounterCombo`) 1)))
      (bind (_output_inputtype _output_attacktype) (break `/Game/Blueprints/Character/ComboConfig` (`|GetArrayItem` (`self.ComboElbow`) _output_get)))
      (if (`|EnumEquality` _output_inputtype InputType)
        (`self.ComboAttack` _output_attacktype InputType)
        (set `self.IsMaybeCombo` false)
        (if (<= (`KismetArrayLibrary.Array_Length` (`self.ComboElbow`)) (`self.CounterCombo`))
          (set `self.CounterCombo` 0)
          (`KismetSystemLibrary.PrintString` "BIG"))
        (else
          (set `self.IsMaybeCombo` false)
          (return)))
      (else
        (set `self.IsMaybeCombo` false)
        (return)))
    (else
      (set `self.IsMaybeCombo` false)
      (return))))

(fn `CheackFlip`
  (params (Direction :type "Float (double-precision)"))
  (`|ExecutionSequence`
    (:`then_0`
      (if (> Direction 0.0)
        (`self.Flip` true)))
    (:`then_1`
      (if (< Direction 0.0)
        (`self.Flip` false)))))

(fn `CheackInputBufferNextCombo`
  (returns (IsReplay :type Boolean))
  (locals (IsReplayBuffer :type Boolean :default true))
  (for (_array_element _array_index) (`self.BufferInput`)
    (bind _output_inputtype (break `/Game/Blueprints/Character/ComboConfig` (`|GetArrayItem` (`self.ComboElbow`) _array_index)))
    (if (not (`|EnumEquality` _array_element _output_inputtype))
      (set `local.IsReplayBuffer` false)))
  (if (`local.IsReplayBuffer`)
    (return true)
    (else
      (return false))))

(fn `ComboAttack`
  (params (AttackType :type "/Game/Blueprints/Enums/AttackType Enum" :default "NewEnumerator3") (InputType :type "/Game/Blueprints/Enums/InputType Enum" :default "NewEnumerator2"))
  (`KismetArrayLibrary.Array_Add` (`self.BufferInput`) InputType)
  (`/Game/Blueprints/Character/BeatEmUpCharacterAnimationBP.ClearAttackAnimation` (`self.Animation`))
  (switch `/Game/Blueprints/Enums/AttackType` AttackType
    (:`NewEnumerator0`
      (set `/Game/Blueprints/Character/BeatEmUpCharacterAnimationBP.IsAttackLeftHand` true (`self.Animation`))
      (set `self.AttackHitBoxBuffer` "NewEnumerator0"))
    (:`NewEnumerator1`
      (set `/Game/Blueprints/Character/BeatEmUpCharacterAnimationBP.IsAttackRightHand` true (`self.Animation`))
      (set `self.AttackHitBoxBuffer` "NewEnumerator1"))
    (:`NewEnumerator2`
      (set `/Game/Blueprints/Character/BeatEmUpCharacterAnimationBP.IsAttackElbow` true (`self.Animation`))
      (set `self.AttackHitBoxBuffer` "NewEnumerator2"))))

(fn `DamageOtherActor`
  (params (Damage :type "Float (double-precision)") (DamagedActor :type "Actor Object Reference"))
  (`GameplayStatics.ApplyDamage` DamagedActor Damage null self))

(fn `DeactiveHitBoxes`
  (`self.ActiveHitBox` "NewEnumerator0")
  (`self.ActiveHitBox` "NewEnumerator1")
  (`self.ActiveHitBox` "NewEnumerator2"))

(fn `Death`
  (if (not (`self.IsDead`))
    (set `self.IsDead` true)
    (`self.DeactiveHitBoxes`)
    (set `self.IsMaybeMoving` false)
    (set `self.IsMaybeAttack` false)
    (set `/Game/Blueprints/Character/BeatEmUpCharacterAnimationBP.IsAttack` false (`self.Animation`))
    (set `/Game/Blueprints/Character/BeatEmUpCharacterAnimationBP.DeadAnimationNumber` (`KismetMathLibrary.RandomIntegerInRange` 0 5) (`self.Animation`))
    (set `/Game/Blueprints/Character/BeatEmUpCharacterAnimationBP.IsDeath` true (`self.Animation`))
    (`PrimitiveComponent.SetCollisionEnabled` (`self.HurtBox`) "NoCollision")
    (`SceneComponent.SetVisibility` (`self.HurtBox`) false false)))

(fn `Flip`
  (params (Flip :type Boolean))
  (bind _mesh (`self.Mesh`))
  (if (!= Flip (`self.IsFlip`))
    (if Flip
      (`SceneComponent.K2_SetRelativeRotation` _mesh (struct :`Yaw` -90.0) false false)
      (set `self.IsFlip` true)
      (else
        (`SceneComponent.K2_SetRelativeRotation` _mesh (struct :`Yaw` 90.0) false false)
        (set `self.IsFlip` false)))))

(fn `GetAnimation`
  (bind _asbeat_em_up_character_animation_bp (cast `/Game/Blueprints/Character/BeatEmUpCharacterAnimationBP` (`SkeletalMeshComponent.GetAnimInstance` (`self.Mesh`))))
  (set `self.Animation` _asbeat_em_up_character_animation_bp))

(fn `ResetCombo`
  (locals (NullBufferAttack :type "Array of /Game/Blueprints/Enums/InputType Enum"))
  (set `self.IsMaybeMoving` true)
  (set `self.IsMaybeAttack` true)
  (`self.DeactiveHitBoxes`)
  (set `self.IsMaybeCombo` false)
  (set `self.CounterCombo` 0)
  (set `self.BufferInput` (`local.NullBufferAttack`)))

(fn `UserConstructionScript`)