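; Player character Blueprint that turns Enhanced Input actions into movement and two-handed attacks.
; On BeginPlay it runs the parent logic, then calls InitInput.
; While IsMaybeMoving is true, Move feeds its axes directly into world X/Y movement and passes the Y value to CheackFlip.
; LeftHand and RightHand inputs share one Attack function, each passing a different enum value.
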(event `self.ReceiveBeginPlay`
  (`parent.ReceiveBeginPlay`)
  (`self.InitInput`))

(event `EnhancedInput|/Game/Blueprints/Input/Actions/Move`
  (params (ActionValue :type "Vector2D Structure") (ElapsedSeconds :type "Float (double-precision)") (TriggeredSeconds :type "Float (double-precision)") (InputAction :type "InputAction Object Reference" :default "/Game/Blueprints/Input/Actions/Move.Move"))
  (:`Triggered`
    (if (`self.IsMaybeMoving`)
      (`self.AddMovementInput` (`KismetMathLibrary.MakeVector` ActionValue_X ActionValue_Y))
      (`self.CheackFlip` ActionValue_Y))))

(event `EnhancedInput|/Game/Blueprints/Input/Actions/LeftHand`
  (params (ActionValue :type Boolean) (ElapsedSeconds :type "Float (double-precision)") (TriggeredSeconds :type "Float (double-precision)") (InputAction :type "InputAction Object Reference" :default "/Game/Blueprints/Input/Actions/LeftHand.LeftHand"))
  (:`Triggered`
    (`self.Attack` "NewEnumerator0")))

(event `EnhancedInput|/Game/Blueprints/Input/Actions/RightHand`
  (params (ActionValue :type Boolean) (ElapsedSeconds :type "Float (double-precision)") (TriggeredSeconds :type "Float (double-precision)") (InputAction :type "InputAction Object Reference" :default "/Game/Blueprints/Input/Actions/RightHand.RightHand"))
  (:`Triggered`
    (`self.Attack` "NewEnumerator1")))

(fn `UserConstructionScript`
  (`parent.UserConstructionScript`))