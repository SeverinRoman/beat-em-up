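; Enemy Blueprint that chases pawns it sees and attacks them at random on arrival.
; Pawn sensing stores the seen pawn as Target when IsMaybeMoving is set, then AIMoveTo follows it to within DistanceStop.
; A successful move triggers one of two Attack variants, picked by coin flip.
; Each tick, while Target is valid, Y velocity feeds CheackFlip to update the enemy's facing.
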(event `self.ReceiveTick`
  (params (DeltaSeconds :type "Float (single-precision)"))
  (`self.RotateEnemy`))

(event `self.Sensing.OnSeePawn`
  (params (Pawn :type "Pawn Object Reference"))
  (if (`self.IsMaybeMoving`)
    (set `self.Target` Pawn)
    (`|AIMoveTo` self (0.0 0.0 0.0) (`self.Target`) (`self.DistanceStop`)
      (:`OnSuccess`
        (`self.RandomAttack`)))))

(fn `RandomAttack`
  (if (`KismetMathLibrary.RandomBool`)
    (`self.Attack` "NewEnumerator0")
    (else
      (`self.Attack` "NewEnumerator1"))))

(fn `RotateEnemy`
  (bind (_returnvalue_x _returnvalue_y) (`KismetMathLibrary.BreakVector` (`self.GetVelocity`)))
  (`/Engine/EditorBlueprintResources/StandardMacros.IsValid` (`self.Target`)
    (:`Is Valid`
      (`self.CheackFlip` _returnvalue_y))))

(fn `UserConstructionScript`
  (`parent.UserConstructionScript`))